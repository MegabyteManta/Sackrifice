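; BP_PlayerSack is a player Blueprint that handles interaction and two key-triggered spawns.
; OverlapCapsule tracks overlapping InteractionInterface implementers, either the actor or its components, in InteractablesInRange.
; The Interact action calls OnInteraction on the first entry, passing itself.
; X spawns a BP_IceBird ahead with random rotation jitter, and E spawns a particle system attached to the Mesh.
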(event OnComponentBeginOverlap(OverlapCapsule)
  (params (OverlappedComponent :type Primitive%20Component%20Object%20Reference) (OtherActor :type Actor%20Object%20Reference) (OtherComp :type Primitive%20Component%20Object%20Reference) (OtherBodyIndex :type Integer) (bFromSweep :type Boolean) (SweepResult :type Hit%20Result%20Structure%20%28by%20ref%29))
  (bind _asinteraction_interface (Utilities|Casting|CastToInteractionInterface OtherActor)
    (:then
      ;[1 1 1] This is scary, checking uniqueness in array?
      (Utilities|Array|AddUnique (Variables|Default|GetInteractablesInRange) _asinteraction_interface))
    (:CastFailed
      (for _array_element (Class|Actor|GetComponentsbyInterface OtherActor "/Game/Blueprints/Dialogue/InteractionInterface.InteractionInterface_C")
        (Utilities|Array|AddUnique (Variables|Default|GetInteractablesInRange) (.AsInteraction%20Interface (Utilities|Casting|CastToInteractionInterface _array_element)))))))

(event OnComponentEndOverlap(OverlapCapsule)
  (params (OverlappedComponent :type Primitive%20Component%20Object%20Reference) (OtherActor :type Actor%20Object%20Reference) (OtherComp :type Primitive%20Component%20Object%20Reference) (OtherBodyIndex :type Integer))
  (bind _asinteraction_interface (Utilities|Casting|CastToInteractionInterface OtherActor)
    (:then
      (Utilities|Array|RemoveItem (Variables|Default|GetInteractablesInRange) _asinteraction_interface))
    (:CastFailed
      (for _array_element (Class|Actor|GetComponentsbyInterface OtherActor "/Game/Blueprints/Dialogue/InteractionInterface.InteractionInterface_C")
        (Utilities|Array|RemoveItem (Variables|Default|GetInteractablesInRange) (.AsInteraction%20Interface (Utilities|Casting|CastToInteractionInterface _array_element)))))))

(event Input|ActionEvents|InputActionInteract
  (params (Key :type Key%20Structure :default "None"))
  (:Pressed
    (if (> (Utilities|Array|Length (Variables|Default|GetInteractablesInRange)) 0)
      (Default|OnInteraction (Utilities|Array|Get(acopy) (Variables|Default|GetInteractablesInRange)) self))))

(event Input|KeyboardEvents|E
  (params (Key :type Key%20Structure :default "None"))
  (bind _mesh (Variables|Character|GetMesh))
  (bind _returnvalue (Transformation|GetWorldTransform _mesh))
  (:Pressed
    (Niagara|SpawnSystemAttached "/Game/Materials/MeshParticles/MeshParticleSystem.MeshParticleSystem" _mesh "None" (.location _returnvalue) (.rotation _returnvalue) "KeepRelativeOffset" false)))

(event Input|KeyboardEvents|X
  (params (Key :type Key%20Structure :default "None"))
  (:Pressed
    (Game|SpawnActorfromClass "/Game/Blueprints/BP_IceBird.BP_IceBird_C" (Math|Transform|MakeTransform (+ (Transformation|GetActorLocation) (* (Transformation|GetActorForwardVector) 100)) (Math|Rotator|CombineRotators (Transformation|GetActorRotation) (Math|Rotator|MakeRotator (Math|Conversions|ToFloat(Integer) (Math|Random|RandomIntegerinRange -15 15)) (Math|Conversions|ToFloat(Integer) (Math|Random|RandomIntegerinRange -15 15)) (Math|Conversions|ToFloat(Integer) (Math|Random|RandomIntegerinRange -15 15)))) "1,1,1") "Undefined" 0 0)))

(fn ConstructionScript)