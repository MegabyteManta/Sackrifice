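; DialogueComponent runs interactive dialogue by using a behavior tree as the conversation logic.
; It spawns a dedicated DialogueAIController on BeginPlay.
; On interaction it shows a dialogue widget with UI-only input and cursor, runs the dialogue tree, and passes the widget to it through the blackboard.
; When the widget fires its exit event, it restores game input, stops the tree and removes the widget.
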(event Custom|OnExit_Event_0
  (bind _dialoguewidget (Variables|Default|GetDialogueWidget))
  (bind _returnvalue (Widget|GetOwningPlayer _dialoguewidget))
  (Input|SetInputModeGameOnly _returnvalue)
  (Variables|/Script/Engine.PlayerController|SetbShowMouseCursor _returnvalue false)
  (AI|Logic|StopLogic (Variables|/Script/AIModule.AIController|GetBrainComponent (Variables|Default|GetAIController)) "Dialogue Exited")
  (Widget|RemovefromParent (Variables|Default|GetDialogueWidget)))

(event EventBeginPlay
  (bind _returnvalue (Game|SpawnActorfromClass "/Game/Blueprints/Dialogue/DialogueAIController.DialogueAIController_C" (Math|Transform|MakeTransform "0, 0, 0" "0, 0, 0" "1,1,1") "Undefined" 0 0))
  (Variables|Default|SetAIController _returnvalue))

(event EventOnInteraction
  (params (PlayerCharacter :type Character%20Object%20Reference))
  (bind _returnvalue (Pawn|GetController PlayerCharacter))
  (bind _asplayer_controller (Utilities|Casting|CastToPlayerController _returnvalue))
  (bind _returnvalue_2 (UserInterface|CreateWidget "/Game/Blueprints/Dialogue/UI_DialogueWidget.UI_DialogueWidget_C" _asplayer_controller))
  (bind _output_get (Variables|Default|SetDialogueWidget _returnvalue_2))
  (EventDispatchers|AssignOnExit _output_get (delegate Custom|OnExit_Event_0))
  (UserInterface|Viewport|AddtoViewport _output_get 0)
  (Input|SetInputModeUIOnly _asplayer_controller _output_get "DoNotLock")
  (Variables|/Script/Engine.PlayerController|SetbShowMouseCursor _asplayer_controller true)
  (AI|RunBehaviorTree (Variables|Default|GetAIController) (Variables|Default|GetDialogueTree))
  (bind _blackboardcomponent (Class|AIController|UseBlackboard (Variables|Default|GetAIController) "/Game/Blueprints/Dialogue/D_DialogueBlackboard.D_DialogueBlackboard"))
  (AI|Components|Blackboard|SetValueasObject _blackboardcomponent (Utilities|Name|MakeLiteralName "DialogueWidget") (Variables|Default|GetDialogueWidget)))